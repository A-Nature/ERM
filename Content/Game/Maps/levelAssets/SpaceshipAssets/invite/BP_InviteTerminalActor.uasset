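; Interactable spaceship invite terminal that offers an "Invite Friends" prompt on E and opens the invite screen through the first-person player controller.
; Interface focus events toggle custom depth on the terminal mesh for highlighting.
; Interacting calls InteractOnServer, which flips InteractToggle and calls InviteTerminalOpen on player controller 0.
; The toggle's OnRep repeats that call, so it targets player 0 wherever the change replicates, not specifically the interacting player.
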(event `/Game/interaction/BI_Interaction.Interface_FocusToggle`
  (params (Focus :type Boolean))
  (`PrimitiveComponent.SetRenderCustomDepth` (`self.inviteTerminal`) Focus))

(event `/Game/interaction/BI_Interaction.Interface_Interact`
  (params (Actor :type "Actor Object Reference"))
  (`self.InteractOnServer`))

(event `InteractOnServer`
  (set `self.InteractToggle` (not (`self.InteractToggle`)))
  (bind _asbp_first_person_player_controller (cast `/Game/Game/Blueprints/BP_FirstPersonPlayerController` (`GameplayStatics.GetPlayerController` 0)))
  (`/Game/Game/Blueprints/BP_FirstPersonPlayerController.InviteTerminalOpen` _asbp_first_person_player_controller))

(fn `GetInteractionWidgetRef`
  (returns (Ref :type "WidgetComponent Object Reference") (Input :type Text) (Description :type Text))
  (return (`self.Widget`) "E" "Invite Friends"))

(fn `OnRep_InteractToggle`
  (bind _asbp_first_person_player_controller (cast `/Game/Game/Blueprints/BP_FirstPersonPlayerController` (`GameplayStatics.GetPlayerController` 0)))
  (`/Game/Game/Blueprints/BP_FirstPersonPlayerController.InviteTerminalOpen` _asbp_first_person_player_controller))

(fn `UserConstructionScript`)