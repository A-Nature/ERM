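; BP_InteractionArea is an interaction area that relays focus changes to its parent actor and toggles that actor's interaction prompt.
; On FocusToggle it stores the state and messages the parent through interface calls, which also return the widget component and prompt text.
; It then sets that component's visibility to match focus and fills the WBP_Interaction widget with input and description text.
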(event `FocusToggle`
  (params (Focused :type Boolean))
  (set `self.Focused` Focused)
  (message `/Game/interaction/BI_Interaction.Interface_FocusToggle` (`self.GetParentActor`) (`self.Focused`))
  (bind (_ref _input _description) (message `/Game/interaction/BI_Interaction.GetInteractionWidgetRef` (`self.GetParentActor`)))
  (`SceneComponent.SetVisibility` _ref (`self.Focused`) true)
  (bind _aswbp_interaction (cast `/Game/interaction/WBP_Interaction` (`WidgetComponent.GetUserWidgetObject` _ref)))
  (`/Game/interaction/WBP_Interaction.SetInteractionText` _aswbp_interaction _input _description))

(event `self.ReceiveBeginPlay`
  (set `self.DefParentActor` (`self.GetParentActor`)))

(fn `UserConstructionScript`)