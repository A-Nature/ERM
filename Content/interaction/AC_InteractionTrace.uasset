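; Actor component that lets a player focus and interact with BP_InteractionArea actors under the camera view.
; Each tick it line-traces from player 0's camera on Visibility and toggles focus on the area hit or lost.
; TryToInteract acts only on zero-duration areas, sending an interface message to the area's parent actor.
; If that parent is a first-person character, InteractOnServer instead calls its PlayerInteract with the owner and location.
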(event `self.ReceiveTick`
  (params (DeltaSeconds :type "Float (single-precision)"))
  (`self.Trace`))

(event `TryToInteract`
  (params (In :type Boolean) (IsToggleable :type Boolean) (InteractingWithPlayer :type Boolean :default false))
  (bind _focusedinteractionarea (`self.FocusedInteractionArea`))
  (bind _focusedinteractionarea_2 (`self.FocusedInteractionArea`))
  (bind _returnvalue (`Actor.GetParentActor` _focusedinteractionarea_2))
  (bind _returnvalue_2 (`Actor.GetParentActor` _focusedinteractionarea))
  (`KismetSystemLibrary.PrintString` (`KismetSystemLibrary.GetDisplayName` (`self.FocusedActor`)))
  (if IsToggleable
    (if In
      (if (`self.IsTracingInteractionArea`)
        (bind _output_get (set `self.Interact Duration` (`/Game/interaction/interactionArea/BP_InteractionArea.InteractDuration` (`self.FocusedInteractionArea`))))
        (if (not (> _output_get 0.0))
          (cast `/Game/Game/Blueprints/BP_FirstPersonCharacter` _returnvalue_2
            (:`then`
              (`self.InteractOnServer` _focusedinteractionarea))
            (:`CastFailed`
              (message `/Game/interaction/BI_Interaction.Interface_Interact` _returnvalue_2 null))))))
    (elif (`self.IsTracingInteractionArea`)
      (bind _output_get_2 (set `self.Interact Duration` (`/Game/interaction/interactionArea/BP_InteractionArea.InteractDuration` (`self.FocusedInteractionArea`))))
      (if (not (> _output_get_2 0.0))
        (cast `/Game/Game/Blueprints/BP_FirstPersonCharacter` _returnvalue
          (:`then`
            (`self.InteractOnServer` _focusedinteractionarea_2))
          (:`CastFailed`
            (message `/Game/interaction/BI_Interaction.Interface_Interact` _returnvalue null)))))))

(event `InteractOnServer`
  (params (InteractionArea :type "/Game/interaction/interactionArea/BP_InteractionArea Object Reference"))
  (bind _asbp_first_person_character (cast `/Game/Game/Blueprints/BP_FirstPersonCharacter` (`Actor.GetParentActor` InteractionArea)))
  (bind _asbp_first_person_character_2 (cast `/Game/Game/Blueprints/BP_FirstPersonCharacter` (`self.GetOwner`)))
  (`/Game/Game/Blueprints/BP_FirstPersonCharacter.PlayerInteract` _asbp_first_person_character (`Actor.K2_GetActorLocation` (`self.GetOwner`)) _asbp_first_person_character_2))

(fn `Trace`
  (bind _returnvalue (`GameplayStatics.GetPlayerCameraManager` 0))
  (bind _returnvalue_2 (`Actor.K2_GetActorLocation` _returnvalue))
  (bind _returnvalue_3 (`KismetMathLibrary.GetForwardVector` (`Actor.K2_GetActorRotation` _returnvalue)))
  (bind (_outhit _returnvalue_4) (`KismetSystemLibrary.LineTraceSingle` (+ _returnvalue_2 (* _returnvalue_3 40.0)) (+ _returnvalue_2 (* _returnvalue_3 (`self.Length`))) "TraceTypeQuery1"))
  (if _returnvalue_4
    (bind (_bblockinghit _binitialoverlap _time _distance _location _impactpoint _normal _impactnormal _physmat _hitactor) (`GameplayStatics.BreakHitResult` _outhit))
    (set `self.FocusedActor` _hitactor)
    (`self.TraceInteractionArea` (== (`GameplayStatics.GetObjectClass` _hitactor) "/Game/interaction/interactionArea/BP_InteractionArea.BP_InteractionArea_C"))
    (else
      (`self.TraceInteractionArea` false))))

(fn `TraceInteractionArea`
  (params (Trace :type Boolean))
  (if Trace
    (if (`self.IsTracingInteractionArea`)
      (`/Game/interaction/interactionArea/BP_InteractionArea.FocusToggle` (`self.FocusedInteractionArea`) false))
    (bind _asbp_interaction_area (cast `/Game/interaction/interactionArea/BP_InteractionArea` (`self.FocusedActor`)))
    (bind _output_get (set `self.FocusedInteractionArea` _asbp_interaction_area))
    (`/Game/interaction/interactionArea/BP_InteractionArea.FocusToggle` _output_get true)
    (set `self.IsTracingInteractionArea` true)
    (elif (`self.IsTracingInteractionArea`)
      (set `self.IsTracingInteractionArea` false)
      (`/Game/interaction/interactionArea/BP_InteractionArea.FocusToggle` (`self.FocusedInteractionArea`) false)
      (set `self.FocusedActor` null)
      (set `self.FocusedInteractionArea` null))))